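; BP_Gems is a collectible gem that stops the HUD timer when the 2D character picks it up.
; Its Box overlap event checks the other actor against 2DCharacterRef, then clears and invalidates the TimerEvent handle on that character's HUD and destroys the gem.
; The graph never assigns 2DCharacterRef, and its BeginPlay, Tick and actor overlap events are disabled stubs.
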(event `self.Box.OnComponentBeginOverlap`
  (params (OverlappedComponent :type "PrimitiveComponent Object Reference") (OtherActor :type "Actor Object Reference") (OtherComp :type "PrimitiveComponent Object Reference") (OtherBodyIndex :type Integer) (bFromSweep :type Boolean) (SweepResult :type "HitResult Structure (by ref)"))
  (bind _2dcharacter_ref (`self.2DCharacter Ref`))
  ; Collect Gem and stop timer
  (if (== OtherActor _2dcharacter_ref)
    (`KismetSystemLibrary.K2_ClearAndInvalidateTimerHandle` (`/Game/UI/WB_HUD.Timer Event` (`/Game/Blueprints/BP_2DCharacter.HUD` _2dcharacter_ref)))
    (`self.K2_DestroyActor`)))

(fn `UserConstructionScript`
  (`parent.UserConstructionScript`))