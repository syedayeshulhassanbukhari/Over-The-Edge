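; BP_MasterSpikes is a Paper2D spike trap that cycles between raised and lowered states and damages actors that touch it.
; BeginPlay runs an endless delay-driven loop that alternates the SpikesDown and SpikesUp events, pausing for a configurable move duration.
; Each event animates by swapping four sprites, then disables the Box collision when down or re-enables it when up.
; Box overlap applies fixed damage to the overlapping actor.
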(event `self.ReceiveBeginPlay`
  ; Begin the move upon event gameplay
  (`parent.ReceiveBeginPlay`)
  (`self.Event SpikesDown` :!label _label)
  (`KismetSystemLibrary.Delay` 0.4)
  (`KismetSystemLibrary.Delay` (`self.Spikes Move Duration`))
  (`self.Event SpikesUp`)
  (`KismetSystemLibrary.Delay` 0.4)
  (`KismetSystemLibrary.Delay` (`self.Spikes Move Duration`))
  (goto _label))

(event `Event SpikesDown`
  ; Enable Moving Spikes Logic
  (`PaperSpriteComponent.SetSprite` (`self.PaperSprite`) "/Game/Assets/Tiles/Sprites/DeathObjects/Sprite/Spikes.Spikes")
  (`KismetSystemLibrary.Delay` (`self.Duration`))
  (`PaperSpriteComponent.SetSprite` (`self.PaperSprite`) "/Game/Assets/Tiles/Sprites/DeathObjects/Sprite/Spikes2.Spikes2")
  (`KismetSystemLibrary.Delay` (`self.Duration`))
  (`PaperSpriteComponent.SetSprite` (`self.PaperSprite`) "/Game/Assets/Tiles/Sprites/DeathObjects/Sprite/Spikes3.Spikes3")
  (`KismetSystemLibrary.Delay` (`self.Duration`))
  (`PaperSpriteComponent.SetSprite` (`self.PaperSprite`) "/Game/Assets/Tiles/Sprites/DeathObjects/Sprite/Spikes4.Spikes4")
  (`PrimitiveComponent.SetCollisionEnabled` (`self.Box`) "NoCollision"))

(event `Event SpikesUp`
  ; Enable Moving Spikes Logic
  (`PaperSpriteComponent.SetSprite` (`self.PaperSprite`) "/Game/Assets/Tiles/Sprites/DeathObjects/Sprite/Spikes4.Spikes4")
  (`KismetSystemLibrary.Delay` (`self.Duration`))
  (`PaperSpriteComponent.SetSprite` (`self.PaperSprite`) "/Game/Assets/Tiles/Sprites/DeathObjects/Sprite/Spikes3.Spikes3")
  (`KismetSystemLibrary.Delay` (`self.Duration`))
  (`PaperSpriteComponent.SetSprite` (`self.PaperSprite`) "/Game/Assets/Tiles/Sprites/DeathObjects/Sprite/Spikes2.Spikes2")
  (`KismetSystemLibrary.Delay` (`self.Duration`))
  (`PaperSpriteComponent.SetSprite` (`self.PaperSprite`) "/Game/Assets/Tiles/Sprites/DeathObjects/Sprite/Spikes.Spikes")
  (`PrimitiveComponent.SetCollisionEnabled` (`self.Box`) "QueryAndPhysics"))

(event `self.Box.OnComponentBeginOverlap`
  (params (OverlappedComponent :type "PrimitiveComponent Object Reference") (OtherActor :type "Actor Object Reference") (OtherComp :type "PrimitiveComponent Object Reference") (OtherBodyIndex :type Integer) (bFromSweep :type Boolean) (SweepResult :type "HitResult Structure (by ref)"))
  ; Apply damage on collision
  (`GameplayStatics.ApplyDamage` OtherActor 1.0))

(fn `UserConstructionScript`
  (`parent.UserConstructionScript`))