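; BP_Turet is a turret actor that automatically fires projectiles at a timed interval.
; After an initial delay on BeginPlay, it calls a custom Fire event that re-triggers itself after each delay, forming an endless loop.
; Each shot spawns a BP_ProjectileObj at the world transform of its Scene component, with the turret as owner.
; It has no targeting or aiming logic.
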(event `self.ReceiveBeginPlay`
  (`parent.ReceiveBeginPlay`)
  (`KismetSystemLibrary.Delay` (`self.Duration`))
  (`self.Event Fire`))

(event `Event Fire`
  (`|SpawnActorFromClass` "/Game/Blueprints/BP_ProjectileObj.BP_ProjectileObj_C" (`SceneComponent.K2_GetComponentToWorld` (`self.Scene`)) "Undefined" "MultiplyWithRoot" self null)
  (`KismetSystemLibrary.Delay` (`self.Duration`))
  (`self.Event Fire`))

(fn `UserConstructionScript`
  (`parent.UserConstructionScript`))