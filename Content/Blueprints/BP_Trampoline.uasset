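; BP_Trampoline is a trampoline that launches the 2D character upward when it enters the box trigger.
; On overlap it overrides the character's vertical velocity through LaunchCharacter and swaps the Paper2D sprite to the raised frame.
; After a configurable delay it restores the idle sprite and fires a reset event that re-arms the DoOnce gate, so it cannot retrigger mid-bounce.
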(event `self.Box.OnComponentBeginOverlap`
  (params (OverlappedComponent :type "PrimitiveComponent Object Reference") (OtherActor :type "Actor Object Reference") (OtherComp :type "PrimitiveComponent Object Reference") (OtherBodyIndex :type Integer) (bFromSweep :type Boolean) (SweepResult :type "HitResult Structure (by ref)"))
  (if (== OtherActor (`self.2DCharacter Ref`))
    (`/Engine/EditorBlueprintResources/StandardMacros.DoOnce` false :!label _label
      (:`Completed`
        (`Character.LaunchCharacter` (`self.2DCharacter Ref`) (`KismetMathLibrary.MakeVector` 0.0 0.0 (`self.Launch Velocity Z`)) false true)
        (`PaperSpriteComponent.SetSprite` (`self.PaperSprite`) "/Game/Assets/Tiles/TramplineUp.TramplineUp")
        (`KismetSystemLibrary.Delay` (`self.Duration to reset Trampoline`))
        (`PaperSpriteComponent.SetSprite` (`self.PaperSprite`) "/Game/Assets/Tiles/TramplineIdle.TramplineIdle")
        (`self.Event Reset Trampoline`)))))

(event `Event Reset Trampoline`
  (goto _label :!via `Reset`))

(fn `UserConstructionScript`
  (`parent.UserConstructionScript`))