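; BP_FallingPlatform is a sprite-based platform that falls after the 2D character enters its box trigger, then respawns.
; A one-time overlap waits a drop delay, adds and activates a Projectile Movement component, and switches the sprite's collision object type to PhysicsBody.
; After a respawn delay it spawns a fresh copy at the location saved on BeginPlay, without destroying itself here.
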(event `self.ReceiveBeginPlay`
  (`parent.ReceiveBeginPlay`)
  (set `self.Starting Location` (`self.K2_GetActorLocation`)))

(event `self.Box.OnComponentBeginOverlap`
  (params (OverlappedComponent :type "PrimitiveComponent Object Reference") (OtherActor :type "Actor Object Reference") (OtherComp :type "PrimitiveComponent Object Reference") (OtherBodyIndex :type Integer) (bFromSweep :type Boolean) (SweepResult :type "HitResult Structure (by ref)"))
  (if (== OtherActor (`self.2DCharacter Ref`))
    (`/Engine/EditorBlueprintResources/StandardMacros.DoOnce` false
      (:`Completed`
        (`KismetSystemLibrary.Delay` (`self.Drop Delay`))
        (bind _returnvalue (`AddComponent|NODE_AddProjectileMovementComponent-0` :`self` self))
        (`ActorComponent.SetActive` _returnvalue true false)
        (`PrimitiveComponent.SetCollisionObjectType` (`self.PaperSprite`) "ECC_PhysicsBody")
        (`KismetSystemLibrary.Delay` (`self.ReSpawn Delay`))
        (`|SpawnActorFromClass` "BP_FallingPlatform_C" (`KismetMathLibrary.Conv_VectorToTransform` (`self.Starting Location`)) "Undefined" "MultiplyWithRoot" null null)))))

(fn `UserConstructionScript`
  (`parent.UserConstructionScript`))