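; BP_Checkpoints is a checkpoint actor for a Paper2D character that updates where the player respawns.
; When the actor held in 2DCharacterRef overlaps the Box component, it writes the Scene component's world location into that character's RespawnLocation.
; The same overlap switches the PaperFlipbook to the Savepoint animation.
; Nothing in the graph assigns the character reference, resets the flipbook or guards against repeat triggers.
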(event `self.Box.OnComponentBeginOverlap`
  (params (OverlappedComponent :type "PrimitiveComponent Object Reference") (OtherActor :type "Actor Object Reference") (OtherComp :type "PrimitiveComponent Object Reference") (OtherBodyIndex :type Integer) (bFromSweep :type Boolean) (SweepResult :type "HitResult Structure (by ref)"))
  (bind _2dcharacter_ref (`self.2DCharacter Ref`))
  (if (== OtherActor _2dcharacter_ref)
    (set `/Game/Blueprints/BP_2DCharacter.Respawn Location` (`SceneComponent.K2_GetComponentLocation` (`self.Scene`)) _2dcharacter_ref)
    (`PaperFlipbookComponent.SetFlipbook` (`self.PaperFlipbook`) "/Game/Assets/Tiles/Sprites/Checkpoints/Flipbooks/Savepoint.Savepoint")))

(fn `UserConstructionScript`
  (`parent.UserConstructionScript`))