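; BP_2DCharacter is a side-scrolling Paper2D player character with horizontal movement, jumping and death on any damage.
; Input drives movement along world X and records the last horizontal direction.
; Tick picks the idle, moving, jump or death flipbook from state, and flips facing through controller yaw, using the recorded direction when stationary.
; Any damage sets the dead flag and deactivates CharacterMovement.
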(event `self.ReceiveTick`
  (params (DeltaSeconds :type "Float (single-precision)"))
  ; Refactor this event Tick
  (`self.Event Handle Animation`)
  (`self.Event Handle Player Rotations`))

(event `InputAction|Jump`
  (params (Key :type "Key Structure"))
  ; Implementing Movements from Inputs
  (:`Pressed`
    (`self.Jump`))
  (:`Released`
    (`self.StopJumping`)))

(event `self.ReceiveAnyDamage`
  (params (Damage :type "Float (single-precision)") (DamageType :type "DamageType Object Reference") (InstigatedBy :type "Controller Object Reference") (DamageCauser :type "Actor Object Reference"))
  (set `self.Is Dead` true)
  (`ActorComponent.SetActive` (`self.CharacterMovement`) false false))

(event `InputAxis|Move`
  (params (AxisValue :type "Float (single-precision)"))
  ; Implementing Movements from Inputs
  ;; Validating moving left or right
  (if (> AxisValue 0.0)
    (set `self.Is Moving Right ?` true)
    (elif (< AxisValue 0.0)
      (set `self.Is Moving Right ?` false)))
  (`self.AddMovementInput` (1.0 0.0 0.0) AxisValue))

(event `Event Handle Animation`
  (bind _sprite (`self.Sprite`))
  ; Handling The movement Animations of Sprites
  (if (`self.Is Dead`)
    (`PaperFlipbookComponent.SetFlipbook` (`self.Sprite`) (`self.Player Death Animation`))
    (elif (`NavMovementComponent.IsFalling` (`self.CharacterMovement`))
      (`PaperFlipbookComponent.SetFlipbook` _sprite "/Game/Assets/Tiles/Characters/Jump.Jump")
      (else
        (`PaperFlipbookComponent.SetFlipbook` _sprite (select `bool` (> (`KismetMathLibrary.VSize` (`MovementComponent.Velocity` (`self.CharacterMovement`))) 0.0) :`false` "/Game/Assets/Tiles/Characters/idle.idle" :`true` "/Game/Assets/Tiles/Characters/Moving.Moving" :!type "PaperFlipbook Object Reference"))))))

(event `Event Handle Player Rotations`
  (bind _velocity_x (`KismetMathLibrary.BreakVector` (`MovementComponent.Velocity` (`self.CharacterMovement`))))
  ; Handling the rotation of the player going left or right
  (`/Engine/EditorBlueprintResources/StandardMacros.CompareFloat` _velocity_x
    (:`>`
      (`Controller.SetControlRotation` (`self.GetController`) (`KismetMathLibrary.MakeRotator` 0.0 0.0 180.0) :!label _label))
    (:`==`
      (if (`self.Is Moving Right ?`)
        (goto _label)
        (else
          (`Controller.SetControlRotation` (`self.GetController`) (`KismetMathLibrary.MakeRotator` 0.0) :!label _label_2))))
    (:`<`
      (goto _label_2))))

(fn `UserConstructionScript`)